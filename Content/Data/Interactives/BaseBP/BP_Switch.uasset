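; BP_Switch is an interactive switch that toggles the visibility of tagged actors when used.
; Trigger01 passes the switch to a Player-tagged actor through AddInteractiveObjMessage on begin overlap and an empty reference on end overlap.
; Interactive calls Switch, which toggles root component visibility on actors matching Tag, without propagating to children.
; If RevealTag is set, it also flips hidden-in-game on actors with that tag.
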(event OnComponentBeginOverlap(Trigger01)
  (params (OverlappedComponent :type Primitive%20Component%20Object%20Reference) (OtherActor :type Actor%20Object%20Reference) (OtherComp :type Primitive%20Component%20Object%20Reference) (OtherBodyIndex :type Integer) (bFromSweep :type Boolean) (SweepResult :type Hit%20Result%20Structure%20%28by%20ref%29))
  ;[1 1 1] OverLap
  (if (Actor|ActorHasTag OtherActor "Player")
    (Class|BPIPlayer|AddInteractiveObj(Message) OtherActor self)))

(event OnComponentEndOverlap(Trigger01)
  (params (OverlappedComponent :type Primitive%20Component%20Object%20Reference) (OtherActor :type Actor%20Object%20Reference) (OtherComp :type Primitive%20Component%20Object%20Reference) (OtherBodyIndex :type Integer))
  ;[1 1 1] OverLap
  (if (Actor|ActorHasTag OtherActor "Player")
    (Class|BPIPlayer|AddInteractiveObj(Message) OtherActor)))

(event Custom|Switch
  (bind _outactors (Actor|GetAllActorswithTag (Variables|Default|GetTag)))
  (for _array_element _outactors
    (Rendering|ToggleVisibility (Variables|/Script/Engine.Actor|GetRootComponent _array_element) false))
  (if (not (== (Variables|Default|GetRevealTag) ""))
    (bind _outactors_2 (Actor|GetAllActorswithTag (Variables|Default|GetRevealTag)))
    (for _array_element_2 _outactors_2
      (Rendering|SetActorHiddenInGame _array_element_2 (not (Variables|/Script/Engine.Actor|GetbHidden _array_element_2))))))

(event EventAddInteractiveObj
  (params (INT_OBJ :type Object%20Object%20Reference)))

(event EventInteractive
  (CallFunction|Switch))

(fn ConstructionScript)