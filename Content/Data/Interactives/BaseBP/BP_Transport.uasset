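; Interactive door that transports the player to a preset location behind a black screen fade.
; Its trigger registers and clears it as the player's interactive object through messages to the overlapping actor tagged Player.
; On interaction it removes movement input, shows the fade widget and swings the door open with a timeline.
; Delays chained off the timeline update then move the player pawn, reset the door and restore input.
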(event OnComponentBeginOverlap(Trigger01)
  (params (OverlappedComponent :type Primitive%20Component%20Object%20Reference) (OtherActor :type Actor%20Object%20Reference) (OtherComp :type Primitive%20Component%20Object%20Reference) (OtherBodyIndex :type Integer) (bFromSweep :type Boolean) (SweepResult :type Hit%20Result%20Structure%20%28by%20ref%29))
  ;[1 1 1] OverLap
  (if (Actor|ActorHasTag OtherActor "Player")
    (Class|BPIPlayer|AddInteractiveObj(Message) OtherActor self)))

(event OnComponentEndOverlap(Trigger01)
  (params (OverlappedComponent :type Primitive%20Component%20Object%20Reference) (OtherActor :type Actor%20Object%20Reference) (OtherComp :type Primitive%20Component%20Object%20Reference) (OtherBodyIndex :type Integer))
  ;[1 1 1] OverLap
  (if (Actor|ActorHasTag OtherActor "Player")
    (Class|BPIPlayer|AddInteractiveObj(Message) OtherActor)))

(event Custom|Transport
  ;[1 1 1] Transport
  (CallFunction|RemoveInputMapping "/Game/Data/InPuts/Player_Movements/IM_Player_Movement.IM_Player_Movement")
  (bind _returnvalue (UserInterface|CreateWidget "/Game/Data/UMG/LS_Interludes/WLS_BlackFade.WLS_BlackFade_C"))
  (bind _output_get (Variables|Default|SetNewVar _returnvalue))
  (UserInterface|Viewport|AddtoViewport _output_get 0)
  (Default|FadeINout _returnvalue)
  (Utilities|FlowControl|FlipFlop
    (:A
      (bind _roatationstrack (Timeline|DoorRoatation Play)
        (:Update
          (Transformation|SetRelativeRotation (Variables|Default|GetDoor) (Math|Rotator|MakeRotator 0.0 0.0 (Math|Float|Lerp 0.0 -9e+01 _roatationstrack)) false false)
          (Utilities|FlowControl|Delay 2.0)
          (Transformation|SetActorLocation (Game|Player|GetPlayerPawn 0) (Variables|Default|GetPlayerLocation) false false)
          (Transformation|SetRelativeRotation (Variables|Default|GetDoor) "0, 0, 0" false false)
          (Utilities|FlowControl|Delay 2.0)
          (CallFunction|AddInputMapping "/Game/Data/InPuts/Player_Movements/IM_Player_Movement.IM_Player_Movement"))))
    (:B
      (Timeline|DoorRoatation PlayFromStart))))

(event EventAddInteractiveObj
  (params (INT_OBJ :type Object%20Object%20Reference))
  ;[1 1 1] Transport
)

(event EventInteractive
  (CallFunction|Transport))

(fn ConstructionScript)