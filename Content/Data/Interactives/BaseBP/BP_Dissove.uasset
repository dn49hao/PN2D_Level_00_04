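; BP_Dissove is an interactive base Blueprint that drives a dissolve-style material effect on a mesh when the player enters its trigger box.
; On overlap by a Player-tagged actor, a timeline lerps a configurable scalar parameter on DisMesh's materials from 1 toward 0.
; On exit it sets the parameter back to 1 immediately and resets the timeline's time without stopping it.
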(event OnComponentBeginOverlap(Trigger_Box)
  (params (OverlappedComponent :type Primitive%20Component%20Object%20Reference) (OtherActor :type Actor%20Object%20Reference) (OtherComp :type Primitive%20Component%20Object%20Reference) (OtherBodyIndex :type Integer) (bFromSweep :type Boolean) (SweepResult :type Hit%20Result%20Structure%20%28by%20ref%29))
  (if (Actor|ActorHasTag OtherActor "Player")
    (bind _roatationstrack (Timeline|Timeline_0 Play)
      (:Update
        (Rendering|Material|SetScalarParameterValueonMaterials (Variables|Default|GetDis_Mesh) (Variables|Default|Get数值名称) (Math|Float|Lerp 1.0 0.0 _roatationstrack))))))

(event OnComponentEndOverlap(Trigger_Box)
  (params (OverlappedComponent :type Primitive%20Component%20Object%20Reference) (OtherActor :type Actor%20Object%20Reference) (OtherComp :type Primitive%20Component%20Object%20Reference) (OtherBodyIndex :type Integer))
  (if (Actor|ActorHasTag OtherActor "Player")
    (Rendering|Material|SetScalarParameterValueonMaterials (Variables|Default|GetDis_Mesh) (Variables|Default|Get数值名称) 1.0)
    (bind _roatationstrack (Timeline|Timeline_0 SetNewTime)
      (:Update
        (Rendering|Material|SetScalarParameterValueonMaterials (Variables|Default|GetDis_Mesh) (Variables|Default|Get数值名称) (Math|Float|Lerp 1.0 0.0 _roatationstrack))))))

(fn ConstructionScript)