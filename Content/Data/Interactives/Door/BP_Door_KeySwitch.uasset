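; Key-locked switch that opens a door by toggling the visibility of every actor carrying a configured tag.
; Its trigger volume registers it as the player's interactive object on overlap and clears it on exit.
; On interaction, it checks the player character for the required item ID and latches an opened flag.
; Once unlocked, later interactions toggle the tagged actors' root components without rechecking the key.
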(event OnComponentBeginOverlap(Trigger01)
  (params (OverlappedComponent :type Primitive%20Component%20Object%20Reference) (OtherActor :type Actor%20Object%20Reference) (OtherComp :type Primitive%20Component%20Object%20Reference) (OtherBodyIndex :type Integer) (bFromSweep :type Boolean) (SweepResult :type Hit%20Result%20Structure%20%28by%20ref%29))
  ;[1 1 1] OverLap
  (if (Actor|ActorHasTag OtherActor "Player")
    (Class|BPIPlayer|AddInteractiveObj(Message) OtherActor self)))

(event OnComponentEndOverlap(Trigger01)
  (params (OverlappedComponent :type Primitive%20Component%20Object%20Reference) (OtherActor :type Actor%20Object%20Reference) (OtherComp :type Primitive%20Component%20Object%20Reference) (OtherBodyIndex :type Integer))
  ;[1 1 1] OverLap
  (if (Actor|ActorHasTag OtherActor "Player")
    (Class|BPIPlayer|AddInteractiveObj(Message) OtherActor)))

(event Custom|Switch
  ;[0.9634 0.9469 1 0.5] 开门检测钥匙逻辑
  (if (Variables|Default|GetbDoorOpened)
    (bind _outactors (Actor|GetAllActorswithTag (Variables|Default|GetTag) :!label _label))
    (for _array_element _outactors
      (Rendering|ToggleVisibility (Variables|/Script/Engine.Actor|GetRootComponent _array_element) false))
    (else
      (bind _asbp_cha_01 (Utilities|Casting|CastToBP_Cha_01 (Game|GetPlayerCharacter 0)))
      (bind _returnvalue (Default|HasItem _asbp_cha_01 (Variables|Default|GetRequiredItemID)))
      (if _returnvalue
        (Variables|Default|SetbDoorOpened true)
        (goto _label)))))

(event EventInteractive
  ;[1 1 1] OverLap
  (CallFunction|Switch))

(fn ConstructionScript)