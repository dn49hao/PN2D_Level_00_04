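; Key-locked interactive door that teleports the player to PlayerLocation, registering itself with the player while they are inside its trigger.
; The first successful interaction consumes the required item from BP_Cha_01 and leaves the door unlocked, while a missing key brings up a dialogue line.
; Transport suspends movement input, runs a black fade and timeline-driven door swing, then uses delays to teleport, reset the door and restore input.
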(event OnComponentBeginOverlap(Trigger01)
  (params (OverlappedComponent :type Primitive%20Component%20Object%20Reference) (OtherActor :type Actor%20Object%20Reference) (OtherComp :type Primitive%20Component%20Object%20Reference) (OtherBodyIndex :type Integer) (bFromSweep :type Boolean) (SweepResult :type Hit%20Result%20Structure%20%28by%20ref%29))
  ;[1 1 1] OverLap
  (if (Actor|ActorHasTag OtherActor "Player")
    (Class|BPIPlayer|AddInteractiveObj(Message) OtherActor self)))

(event OnComponentEndOverlap(Trigger01)
  (params (OverlappedComponent :type Primitive%20Component%20Object%20Reference) (OtherActor :type Actor%20Object%20Reference) (OtherComp :type Primitive%20Component%20Object%20Reference) (OtherBodyIndex :type Integer))
  ;[1 1 1] OverLap
  (if (Actor|ActorHasTag OtherActor "Player")
    (Class|BPIPlayer|AddInteractiveObj(Message) OtherActor)))

(event Custom|Transport
  ;[1 1 1] 拾取钥匙出门
  (if (Variables|Default|GetbDoorOpened)
    (CallFunction|RemoveInputMapping "/Game/Data/InPuts/Player_Movements/IM_Player_Movement.IM_Player_Movement" :!label _label)
    (bind _returnvalue (UserInterface|CreateWidget "/Game/Data/UMG/LS_Interludes/WLS_BlackFade.WLS_BlackFade_C"))
    (bind _output_get (Variables|Default|SetNewVar _returnvalue))
    (UserInterface|Viewport|AddtoViewport _output_get 0)
    (Default|FadeINout _returnvalue)
    (Utilities|FlowControl|FlipFlop
      (:A
        (bind _roatationstrack (Timeline|DoorRoatation Play)
          (:Update
            (Transformation|SetRelativeRotation (Variables|Default|GetDoor) (Math|Rotator|MakeRotator 0.0 0.0 (Math|Float|Lerp 0.0 -9e+01 _roatationstrack)) false false)
            (Utilities|FlowControl|Delay 2.0)
            (Transformation|SetActorLocation (Game|Player|GetPlayerPawn 0) (Variables|Default|GetPlayerLocation) false true)
            (Transformation|SetRelativeRotation (Variables|Default|GetDoor) "0, 0, 0" false false)
            (Utilities|FlowControl|Delay 2.0)
            (CallFunction|AddInputMapping "/Game/Data/InPuts/Player_Movements/IM_Player_Movement.IM_Player_Movement"))))
      (:B
        (Timeline|DoorRoatation PlayFromStart)))
    (else
      (bind _asbp_cha_01 (Utilities|Casting|CastToBP_Cha_01 (Game|GetPlayerCharacter 0)))
      (bind _returnvalue_2 (Default|HasItem _asbp_cha_01 (Variables|Default|GetRequiredItemID)))
      (if _returnvalue_2
        (bind _asbp_cha_01_2 (Utilities|Casting|CastToBP_Cha_01 (Game|GetPlayerCharacter 0)))
        (Default|RemoveItem _asbp_cha_01_2 (Variables|Default|GetRequiredItemID))
        (Variables|Default|SetbDoorOpened true)
        (goto _label)
        (else
          (bind _asbp_cha_01_3 (Utilities|Casting|CastToBP_Cha_01 (Game|GetPlayerCharacter 0)))
          (Utilities|IsValid (Variables|/Game/Assests/Charactors/C_01/BP/BP_Cha_01.BP_Cha_01_C|GetDialogueUI _asbp_cha_01_3)
            (:Is%20Not%20Valid
              (bind _returnvalue_3 (UserInterface|CreateWidget "/Game/Data/UMG/Dialogue/WBP_DialogueBox.WBP_DialogueBox_C"))
              (bind _asbp_cha_01_4 (Utilities|Casting|CastToBP_Cha_01 (Game|GetPlayerCharacter 0)))
              (bind _output_get_2 (Variables|/Game/Assests/Charactors/C_01/BP/BP_Cha_01.BP_Cha_01_C|SetDialogueUI _asbp_cha_01_4 _returnvalue_3))
              (Default|ShowLine _output_get_2 (Variables|Default|GetSpeaker) (Variables|Default|GetInText))
              (UserInterface|Viewport|AddtoViewport _returnvalue_3 0)
              (Utilities|FlowControl|Delay 0.0)
              (Default|ShowPanel _returnvalue_3))))))))

(event EventInteractive
  ;[1 1 1] OverLap
  (CallFunction|Transport))

(fn ConstructionScript)