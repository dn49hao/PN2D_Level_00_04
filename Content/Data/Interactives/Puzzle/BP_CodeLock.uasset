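; BP_CodeLock is an interactive code lock puzzle object that opens a keypad-style lock UI for the player until solved.
; Its trigger overlap registers it as the player's interactive object and toggles the icon mesh and interaction prompts.
; On interaction, if no examine UI is open, it creates WBP_CodeLock, stores it on BP_Cha_01 and shows the panel after a zero-length delay.
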(event OnComponentBeginOverlap(Trigger01)
  (params (OverlappedComponent :type Primitive%20Component%20Object%20Reference) (OtherActor :type Actor%20Object%20Reference) (OtherComp :type Primitive%20Component%20Object%20Reference) (OtherBodyIndex :type Integer) (bFromSweep :type Boolean) (SweepResult :type Hit%20Result%20Structure%20%28by%20ref%29))
  ;[1 1 1] OverLap
  (if (Actor|ActorHasTag OtherActor "Player")
    (if (not (Variables|Default|GetbSolved))
      (Class|BPIPlayer|AddInteractiveObj(Message) OtherActor self)
      (bind _asbp_cha_01 (Utilities|Casting|CastToBP_Cha_01 OtherActor))
      (Default|ShowExamineIcon _asbp_cha_01)
      (Rendering|SetVisibility (Variables|Default|GetIconMesh) true true)
      (Default|ShowPlayerInteractIcon _asbp_cha_01))))

(event OnComponentEndOverlap(Trigger01)
  (params (OverlappedComponent :type Primitive%20Component%20Object%20Reference) (OtherActor :type Actor%20Object%20Reference) (OtherComp :type Primitive%20Component%20Object%20Reference) (OtherBodyIndex :type Integer))
  ;[1 1 1] OverLap
  (if (Actor|ActorHasTag OtherActor "Player")
    (Class|BPIPlayer|AddInteractiveObj(Message) OtherActor)
    (Rendering|SetVisibility (Variables|Default|GetIconMesh) false true)
    (bind _asbp_cha_01 (Utilities|Casting|CastToBP_Cha_01 OtherActor))
    (Default|HidePlayerInteractIcon _asbp_cha_01)))

(event EventBeginPlay
  ;[1 1 1 0.5] icon逻辑
  (Rendering|SetVisibility (Variables|Default|GetIconMesh) false true))

(event EventInteractive
  ;[0.9325 0.8849 1 0.5] Comment【密码锁】
  (if (not (Variables|Default|GetbSolved))
    (bind _asbp_cha_01 (Utilities|Casting|CastToBP_Cha_01 (Game|GetPlayerCharacter 0)))
    (Utilities|IsValid (Variables|/Game/Assests/Charactors/C_01/BP/BP_Cha_01.BP_Cha_01_C|GetExamine%20UI _asbp_cha_01)
      (:Is%20Not%20Valid
        (bind _returnvalue (UserInterface|CreateWidget "/Game/Data/UMG/Puzzle/WBP_CodeLock.WBP_CodeLock_C" (Game|GetPlayerController 0)))
        (Variables|/Game/Assests/Charactors/C_01/BP/BP_Cha_01.BP_Cha_01_C|SetCodeLock%20UI _asbp_cha_01 _returnvalue)
        (Variables|/Game/Data/UMG/Puzzle/WBP_CodeLock.WBP_CodeLock_C|SetOwnerLock _returnvalue 0)
        (UserInterface|Viewport|AddtoViewport _returnvalue 0)
        (Utilities|FlowControl|Delay 0.0)
        (Default|ShowPanel _returnvalue)))))

(fn ConstructionScript)