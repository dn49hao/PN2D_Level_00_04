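; BP_Item_Key is an interactive key pickup that asks the player to confirm before taking it.
; Its trigger registers it as the player's interactive object and shows a pickup icon, clearing both on exit.
; Interacting opens WBP_PickupConfirm with the item's description, links widget, key and BP_Cha_01, and changes player status while keeping game-only input without a cursor.
; Collision is disabled at BeginPlay if the key starts hidden.
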(event OnComponentBeginOverlap(Trigger01)
  (params (OverlappedComponent :type Primitive%20Component%20Object%20Reference) (OtherActor :type Actor%20Object%20Reference) (OtherComp :type Primitive%20Component%20Object%20Reference) (OtherBodyIndex :type Integer) (bFromSweep :type Boolean) (SweepResult :type Hit%20Result%20Structure%20%28by%20ref%29))
  ;[1 1 1] OverLap
  (if (Actor|ActorHasTag OtherActor "Player")
    (Class|BPIPlayer|AddInteractiveObj(Message) OtherActor self)
    (bind _asbp_cha_01 (Utilities|Casting|CastToBP_Cha_01 OtherActor))
    (Default|ShowPickupIcon _asbp_cha_01)))

(event OnComponentEndOverlap(Trigger01)
  (params (OverlappedComponent :type Primitive%20Component%20Object%20Reference) (OtherActor :type Actor%20Object%20Reference) (OtherComp :type Primitive%20Component%20Object%20Reference) (OtherBodyIndex :type Integer))
  ;[1 1 1] OverLap
  (if (Actor|ActorHasTag OtherActor "Player")
    (Class|BPIPlayer|AddInteractiveObj(Message) OtherActor)
    (bind _asbp_cha_01 (Utilities|Casting|CastToBP_Cha_01 OtherActor))
    (Default|HideInteractIcons _asbp_cha_01)))

(event Custom|Switch
  (bind _returnvalue (Game|GetPlayerController 0))
  ;[0.02089 0.01234 0.15 0.5] 钥匙逻辑
  (if (not (Variables|Default|GetbWaitingConfirm))
    (Variables|Default|SetbWaitingConfirm false)
    (bind _returnvalue_2 (UserInterface|CreateWidget "/Game/Data/UMG/HUD/WBP_PickupConfirm.WBP_PickupConfirm_C" (Game|GetPlayerController 0)))
    (UserInterface|CreateWidget "/Game/Data/UMG/HUD/WBP_PickupConfirm.WBP_PickupConfirm_C")
    (bind _asbp_cha_01 (Utilities|Casting|CastToBP_Cha_01 (Game|GetPlayerCharacter 0)))
    (Variables|/Game/Assests/Charactors/C_01/BP/BP_Cha_01.BP_Cha_01_C|SetPickup%20Confirm%20UI _asbp_cha_01 _returnvalue_2)
    (Default|SetupPrompt _returnvalue_2 "Pick Up?" (Variables|Default|GetItem%20Description) "/Game/Data/UMG/Textures/key.key")
    (Default|HideInteractIcons _asbp_cha_01)
    (Variables|/Game/Data/UMG/HUD/WBP_PickupConfirm.WBP_PickupConfirm_C|SetSourcePickup _returnvalue_2 self)
    ;;[0.15 0.003906 0.003906 0.5] 显示鼠标-由鼠标控制面板菜单【勾选关闭】
    (UserInterface|Viewport|AddtoViewport _returnvalue_2 0)
    (Variables|/Script/Engine.PlayerController|SetbShowMouseCursor _returnvalue false)
    (Input|SetInputModeGameOnly _returnvalue false)
    (Input|SetIgnoreMoveInput _returnvalue false)
    (Variables|/Game/Assests/Charactors/C_01/BP/BP_Cha_01.BP_Cha_01_C|SetPlayerStatus _asbp_cha_01 "NewEnumerator3")))

(event EventBeginPlay
  ;[0.02089 0.01234 0.15 0.5] 钥匙逻辑
  ;;[0.15 0.15 0.15 0.5] 开始隐藏碰撞
  (if (Variables|Rendering|GetbHidden)
    (Collision|SetActorEnableCollision false)))

(event EventInteractive
  ;[1 1 1] OverLap
  (CallFunction|Switch))

(fn ConstructionScript)