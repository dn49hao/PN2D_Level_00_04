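; Player character for a side-view game with sprite movement along X, sprint, flashlight and a spawned camera actor that follows it each tick.
; Holds an eight-slot inventory as parallel arrays, with add, remove and clear functions that refresh the inventory HUD.
; Move and interact inputs are routed by player status and open UI to inventory, dialogue, examine, code lock, pickup confirmation or the current interactable.
; Also toggles examine and pickup prompt icons.
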(event Custom|SayBagFull
  ;[0.7872 0.4547 1 0.5] Inventory-背包
  ;;[0.1981 0.162 0.1046] 【拾取物品到最后格时判断背包是否已满，如满弹出提示】
  (Utilities|IsValid (Variables|交互UI|GetDialogueUI)
    (:Is%20Not%20Valid
      (bind _returnvalue (UserInterface|CreateWidget "/Game/Data/UMG/Dialogue/WBP_DialogueBox.WBP_DialogueBox_C" (Game|GetPlayerController 0)))
      (Variables|交互UI|SetDialogueUI _returnvalue)
      (Default|ShowLine _returnvalue "" "背包满了，我没有办法拿更多的东西了")
      (UserInterface|Viewport|AddtoViewport _returnvalue 0)
      (Utilities|FlowControl|Delay 0.0)
      (Default|ShowPanel _returnvalue))))

(event Input|EnhancedActionEvents|EnhancedInputActionIA_movement
  (params (ActionValue :type Float%20%28double-precision%29) (ElapsedSeconds :type Float%20%28double-precision%29) (TriggeredSeconds :type Float%20%28double-precision%29) (InputAction :type Input%20Action%20Object%20Reference :default "/Game/Data/InPuts/Player_Movements/IA_movement.IA_movement"))
  (bind _pointlight (Variables|Default|GetPointLight))
  (bind _inventoryhud (Variables|背包|GetInventoryHUD))
  ;[1 1 1] Movements-玩家行为
  (:Triggered
    ;;[0.15 0.003125 0.003125 0.5] 开启背包移动行为锁定
    (Variables|玩家基础|SetPlayerForward ActionValue)
    (if (Utilities|Enum|Equal(Enum) (Variables|玩家基础|GetPlayerStatus) "NewEnumerator3")
      (switch Utilities|FlowControl|Switch|SwitchonPlayerStatus (Variables|玩家基础|GetPlayerStatus) :!label _label
        (:NewEnumerator0
          (Pawn|Input|AddMovementInput "1.000000,0.000000,0.000000" (Variables|玩家基础|GetPlayerForward) false :!label _label_2)
          (Transformation|SetRelativeRotation (Variables|Default|GetSprite) (Math|Rotator|MakeRotator 0.0 0.0 (* (- (Variables|玩家基础|GetPlayerForward) 1.0) 9e+01)) false false)
          (if (== (.x (Variables|/Script/Engine.MovementComponent|GetVelocity (Variables|Character|GetCharacterMovement))) 0.0)
            (Transformation|SetRelativeLocation _pointlight (Math|Vector|MakeVector 0.0 13.0 3e+01) false false :!label _label_3)
            (else
              (Transformation|SetRelativeLocation _pointlight (Math|Vector|MakeVector (* (Variables|玩家基础|GetPlayerForward) 2e+01) 13.0 3e+01) false false))))
        (:NewEnumerator1
          (goto _label_2))
        (:NewEnumerator2
          (goto _label_2))
        (:NewEnumerator3
          ;;[0.15 0.008594 0.008594 0.5] 拾取UI
          (Utilities|IsValid (Variables|交互UI|GetPickup%20Confirm%20UI)
            (:Is%20Valid
              (if (< (Variables|玩家基础|GetPlayerForward) -0.5)
                (Default|SelectYes (Variables|交互UI|GetPickup%20Confirm%20UI))
                (elif (> (Variables|玩家基础|GetPlayerForward) 0.5)
                  (Default|SelectNo (Variables|交互UI|GetPickup%20Confirm%20UI))))))))
      (else
        (bind _b_handled (CallFunction|TryInventoryNav))
        (if _b_handled
          (Variables|玩家基础|SetPlayerStatus "NewEnumerator0")
          (else
            (goto _label))))))
  (:Completed
    (Utilities|IsValid _inventoryhud
      (:Is%20Valid
        (if (Variables|/Game/Data/UMG/HUD/WBP_InventoryHUD.WBP_InventoryHUD_C|GetInventoryVisible _inventoryhud)
          (Variables|/Game/Data/UMG/HUD/WBP_InventoryHUD.WBP_InventoryHUD_C|SetSlot%20Nav%20Latched _inventoryhud false)
          (Variables|/Game/Data/UMG/HUD/WBP_InventoryHUD.WBP_InventoryHUD_C|SetSlot%20Menu%20Latched _inventoryhud false)
          (goto _label_3))))))

(event Input|EnhancedActionEvents|EnhancedInputActionIA_Sprint
  (params (ActionValue :type Boolean) (ElapsedSeconds :type Float%20%28double-precision%29) (TriggeredSeconds :type Float%20%28double-precision%29) (InputAction :type Input%20Action%20Object%20Reference :default "/Game/Data/InPuts/Player_Movements/IA_Sprint.IA_Sprint"))
  (bind _charactermovement (Variables|Character|GetCharacterMovement))
  ;[1 1 1] Movements-玩家行为
  ;;[1 1 1] 对话
  (:Triggered
    ;;;[0.15 0 0 0.5] 先判断是否进入对话
    (if (not (Utilities|Enum|Equal(Enum) (Variables|玩家基础|GetPlayerStatus) "NewEnumerator3"))
      (Variables|/Script/Engine.CharacterMovementComponent|SetMaxWalkSpeed _charactermovement 3e+02)
      (Variables|玩家基础|SetPlayerStatus "NewEnumerator2")))
  (:Completed
    (if (not (Utilities|Enum|Equal(Enum) (Variables|玩家基础|GetPlayerStatus) "NewEnumerator3"))
      (Variables|/Script/Engine.CharacterMovementComponent|SetMaxWalkSpeed _charactermovement 1.2e+02)
      (Variables|玩家基础|SetPlayerStatus "NewEnumerator1"))))

(event Input|EnhancedActionEvents|EnhancedInputActionIA_Flashlight
  (params (ActionValue :type Boolean) (ElapsedSeconds :type Float%20%28double-precision%29) (TriggeredSeconds :type Float%20%28double-precision%29) (InputAction :type Input%20Action%20Object%20Reference :default "/Game/Data/InPuts/Player_Movements/IA_Flashlight.IA_Flashlight"))
  ;[1 1 1] Movements-玩家行为
  ;;[1 1 1] 手电筒开关
  (:Started
    ;;;[0.15 0 0 0.5] 先判断是否进入对话
    (if (not (Utilities|Enum|Equal(Enum) (Variables|玩家基础|GetPlayerStatus) "NewEnumerator3"))
      (Rendering|ToggleVisibility (Variables|Default|GetSpotLight) false))))

(event Input|EnhancedActionEvents|EnhancedInputActionIA_Interactive
  (params (ActionValue :type Boolean) (ElapsedSeconds :type Float%20%28double-precision%29) (TriggeredSeconds :type Float%20%28double-precision%29) (InputAction :type Input%20Action%20Object%20Reference :default "/Game/Data/InPuts/Player_Movements/IA_Interactive.IA_Interactive"))
  (bind _codelock_ui (Variables|交互UI|GetCodeLock%20UI))
  (bind _pickup_confirm_ui (Variables|交互UI|GetPickup%20Confirm%20UI))
  (bind _inventoryhud (Variables|背包|GetInventoryHUD))
  ;[0.3498 0.3198 1] Interactive-交互
  (Utilities|IsValid _inventoryhud
    (:Is%20Valid
      (if (Variables|/Game/Data/UMG/HUD/WBP_InventoryHUD.WBP_InventoryHUD_C|GetInventoryVisible (Variables|背包|GetInventoryHUD))
        ;;[0.15 0 0 0.5] 按下J弹出选单
        (Default|HandleInventoryJ _inventoryhud)
        (else
          (Utilities|IsValid (Variables|交互UI|GetDialogueUI) :!label _label
            (:Is%20Valid
              (Default|HandleInteractive (Variables|交互UI|GetDialogueUI)))
            (:Is%20Not%20Valid
              (Utilities|IsValid (Variables|交互UI|GetExamine%20UI)
                (:Is%20Valid
                  (Default|HandleExamine (Variables|交互UI|GetExamine%20UI)))
                (:Is%20Not%20Valid
                  ;;[0.06125 0.06125 0.06125] 开启密码锁
                  (Utilities|IsValid _codelock_ui
                    (:Is%20Valid
                      (Default|HandleCodeLock _codelock_ui))
                    (:Is%20Not%20Valid
                      ;;[0.15 0.15 0.15 0.5] 开着板时判断不要再 Create
                      (Utilities|IsValid _pickup_confirm_ui
                        (:Is%20Valid
                          (Default|ConfirmChoice _pickup_confirm_ui))
                        (:Is%20Not%20Valid
                          (Utilities|IsValid (Variables|交互UI|GetINT%20OBJ)
                            (:Is%20Valid
                              (bind _int_obj (Variables|交互UI|GetINT%20OBJ)
                                (:then
                                  (Class|BPIPlayer|Interactive(Message) _int_obj))
                                (:else)))))))))))))))
    (:Is%20Not%20Valid
      (goto _label))))

(event Input|EnhancedActionEvents|EnhancedInputActionIA_Inventory
  (params (ActionValue :type Boolean) (ElapsedSeconds :type Float%20%28double-precision%29) (TriggeredSeconds :type Float%20%28double-precision%29) (InputAction :type Input%20Action%20Object%20Reference :default "/Game/Data/InPuts/Player_Movements/IA_Inventory.IA_Inventory"))
  ;[0.7872 0.4547 1 0.5] Inventory-背包
  ;;[0.06582 0.1906 0.7865 0.5] 按下I键开启或关闭HUD
  (:Started
    (if (not (Utilities|Enum|Equal(Enum) (Variables|玩家基础|GetPlayerStatus) "NewEnumerator3"))
      (Utilities|IsValid (Variables|背包|GetInventoryHUD)
        (:Is%20Valid
          (Default|ToggleInventoryHUD (Variables|背包|GetInventoryHUD)))))))

(event EventBeginPlay
  ;[0.7872 0.4547 1 0.5] Inventory-背包
  ;;[0.06682 0.15 0.1112 0.5] 主逻辑
  (CallFunction|HideInteractIcons)
  (bind _returnvalue (UserInterface|CreateWidget "/Game/Data/UMG/HUD/WBP_InventoryHUD.WBP_InventoryHUD_C" (Game|GetPlayerController 0)))
  (bind _output_get (Variables|背包|SetInventoryHUD _returnvalue))
  ;;;[0.999 0.8342 0.2555] Inventory HUD → HideInventoryHUD
  (UserInterface|Viewport|AddtoViewport _output_get 0)
  (Default|HideInventoryHUD _output_get)
  ;;;[0.15 0.0234 0.1385 0.5] Inventory数组（格子）
  (Utilities|Array|Resize (Variables|背包|GetInventoryItems) 8)
  (Utilities|Array|Resize (Variables|背包|GetInventory%20Descs) 8)
  (Utilities|Array|Resize (Variables|背包|GetInventory%20Titles) 8)
  (Utilities|Array|Resize (Variables|背包|GetInventory%20Can%20Use) 8)
  (Utilities|Array|Resize (Variables|背包|GetInventory%20Can%20Discard) 8)
  ;;;[0.06125 0.009134 0.05613] 显示图片
  (Utilities|Array|Resize (Variables|背包|GetInventory%20Images) 8)
  (Default|RefreshInventory _output_get)
  (bind _returnvalue_2 (Game|SpawnActorfromClass "/Game/Assests/Charactors/C_01/BP/BP_Camera_01.BP_Camera_01_C" (Math|Transform|MakeTransform (Transformation|GetActorLocation) "0, 0, 0" "1.000000,1.000000,1.000000") "AlwaysSpawn" "MultiplyWithRoot" 0 0))
  (bind _output_get_2 (Variables|玩家基础|SetPlayer_Camera_01 _returnvalue_2))
  (Game|Player|SetViewTargetwithBlend (Game|GetPlayerController 0) _output_get_2 0.0 "VTBlend_Linear" 0.0 false)
  (CallFunction|AddInputMapping "/Game/Data/InPuts/Player_Movements/IM_Player_Movement.IM_Player_Movement"))

(event EventAddInteractiveObj
  (params (INT_OBJ :type Object%20Object%20Reference))
  ;[0.3498 0.3198 1] Interactive-交互
  (Variables|交互UI|SetINT%20OBJ INT_OBJ))

(event EventTick
  (params (DeltaSeconds :type Float%20%28single-precision%29))
  ;[0.3498 0.3198 1] Interactive-交互
  ;;[0.121 0.9203 1] Camera location
  (Transformation|SetActorLocation (Variables|玩家基础|GetPlayer_Camera_01) (Transformation|GetActorLocation) false false))

(fn ConstructionScript)

(fn HasItem
  (params (ItemID :type Name))
  (return (Utilities|Array|ContainsItem (Variables|背包|GetInventoryItems) ItemID)))

(fn AddItem
  (params (ItemID :type Name) (In%20Image :type Texture%202D%20Object%20Reference) (In%20Desc :type Text) (In%20Title :type Text) (In%20Can%20Use :type Boolean) (In%20Can%20Discard :type Boolean))
  (bind _inventoryhud (Variables|背包|GetInventoryHUD))
  (if (!= ItemID "")
    (for _index (range 0 7)
      (if (== (Utilities|Array|Get(acopy) (Variables|背包|GetInventoryItems) _index) "")
        (Utilities|Array|SetArrayElem (Variables|背包|GetInventoryItems) _index ItemID)
        (Utilities|Array|SetArrayElem (Variables|背包|GetInventory%20Titles) _index In%20Title)
        (Utilities|Array|SetArrayElem (Variables|背包|GetInventory%20Descs) _index In%20Desc)
        (Utilities|Array|SetArrayElem (Variables|背包|GetInventory%20Can%20Use) _index In%20Can%20Use)
        (Utilities|Array|SetArrayElem (Variables|背包|GetInventory%20Can%20Discard) _index In%20Can%20Discard)
        (Utilities|Array|SetArrayElem (Variables|背包|GetInventory%20Images) _index In%20Image)
        (Utilities|IsValid _inventoryhud
          (:Is%20Valid
            (Default|RefreshInventory _inventoryhud))
          (:Is%20Not%20Valid
            _))
        (return true)))
    (return false)
    (else
      (return false))))

(fn RemoveItem
  (params (ItemID :type Name))
  (bind _inventoryitems (Variables|背包|GetInventoryItems))
  (bind _inventoryhud (Variables|背包|GetInventoryHUD))
  (for _index (range 0 7)
    (if (== (Utilities|Array|Get(acopy) _inventoryitems _index) ItemID)
      (Utilities|Array|SetArrayElem _inventoryitems _index "")
      (Utilities|Array|SetArrayElem (Variables|背包|GetInventory%20Descs) _index "")
      (Utilities|Array|SetArrayElem (Variables|背包|GetInventory%20Can%20Use) _index false)
      (Utilities|Array|SetArrayElem (Variables|背包|GetInventory%20Can%20Discard) _index false)
      (Utilities|Array|SetArrayElem (Variables|背包|GetInventory%20Images) _index 0)
      (Utilities|IsValid _inventoryhud
        (:Is%20Valid
          (Default|RefreshInventory _inventoryhud))
        (:Is%20Not%20Valid
          _))
      (return))))

(fn ShowPlayerInteractIcon
  (Rendering|SetVisibility (Variables|Default|GetCheck_UI) true false))

(fn HidePlayerInteractIcon
  (Rendering|SetVisibility (Variables|Default|GetCheck_UI) false false))

(fn ShowExamineIcon
  (Rendering|SetVisibility (Variables|Default|GetCheck_UI) true false)
  (Rendering|SetVisibility (Variables|Default|GetPickup_UI) false false))

(fn ShowPickupIcon
  (Rendering|SetVisibility (Variables|Default|GetPickup_UI) true false)
  (Rendering|SetVisibility (Variables|Default|GetCheck_UI) false false))

(fn HideInteractIcons
  (Rendering|SetVisibility (Variables|Default|GetCheck_UI) false false)
  (Rendering|SetVisibility (Variables|Default|GetPickup_UI) false false))

(fn TryInventoryNav
  (bind _inventoryhud (Variables|背包|GetInventoryHUD))
  (Utilities|IsValid "/Game/Data/UMG/HUD/WBP_InventoryHUD.WBP_InventoryHUD"
    (:Is%20Valid
      (if (Variables|/Game/Data/UMG/HUD/WBP_InventoryHUD.WBP_InventoryHUD_C|GetInventoryVisible _inventoryhud)
        (if (Variables|/Game/Data/UMG/HUD/WBP_InventoryHUD.WBP_InventoryHUD_C|GetSlot%20Menu%20Visible _inventoryhud)
          (Default|HandleSlotMenuNav (Variables|背包|GetInventoryHUD) (Variables|玩家基础|GetPlayerForward))
          (return true)
          (else
            (Utilities|IsValid (Variables|/Game/Data/UMG/HUD/WBP_InventoryHUD.WBP_InventoryHUD_C|GetInv%20Examine%20UI _inventoryhud)
              (:Is%20Valid
                (return true))
              (:Is%20Not%20Valid
                (Default|HandleInventoryNav (Variables|背包|GetInventoryHUD) (Variables|玩家基础|GetPlayerForward))
                (return true)))))
        (else
          (return false))))
    (:Is%20Not%20Valid
      (return false))))

(fn ClearSlot
  (params (Slot%20Index :type Integer))
  (bind _inventoryhud (Variables|背包|GetInventoryHUD))
  (if (or (< Slot%20Index 0) (> Slot%20Index 7))
    (return)
    (else
      (Utilities|Array|SetArrayElem (Variables|背包|GetInventory%20Images) Slot%20Index 0)
      (Utilities|Array|SetArrayElem (Variables|背包|GetInventory%20Can%20Discard) Slot%20Index false)
      (Utilities|Array|SetArrayElem (Variables|背包|GetInventory%20Can%20Use) Slot%20Index false)
      (Utilities|Array|SetArrayElem (Variables|背包|GetInventory%20Descs) Slot%20Index "")
      (Utilities|Array|SetArrayElem (Variables|背包|GetInventoryItems) Slot%20Index "")
      (Utilities|Array|SetArrayElem (Variables|背包|GetInventory%20Titles) Slot%20Index "")
      (Utilities|IsValid _inventoryhud
        (:Is%20Valid
          (Default|RefreshInventory _inventoryhud))
        (:Is%20Not%20Valid
          (return))))))